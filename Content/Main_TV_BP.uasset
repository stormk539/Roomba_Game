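; TV actor that changes its screen materials based on the player character's TvPress flag.
; Every Tick casts the player to ThirdPersonCharacter and runs a while loop on TvPress, setting empty materials on Plane and SMTV1B, each followed by a Delay.
; The loop's exit sets Plane to a black lacquered wood material.
; The loop relies on latent Delays that cannot pause it, and the news-material branch is unconnected.
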(event `self.ReceiveTick`
  (params (DeltaSeconds :type "Float (single-precision)"))
  (bind _asthird_person_character (cast `/Game/GameFolder/Blueprints/CharacterBlueprints/ThirdPersonCharacter1` (`GameplayStatics.GetPlayerCharacter` 0)))
  (while (`/Game/GameFolder/Blueprints/CharacterBlueprints/ThirdPersonCharacter1.Tv_Press` _asthird_person_character)
    (`|ExecutionSequence`
      (:`then_0`
        (`PrimitiveComponent.SetMaterial` (`self.Plane`) 0 null)
        (`KismetSystemLibrary.Delay` 5.0))
      (:`then_1`
        (`PrimitiveComponent.SetMaterial` (`self.SM_TV_1B`) 0 null)
        (`KismetSystemLibrary.Delay` 5.0))))
  (`PrimitiveComponent.SetMaterial` (`self.Plane`) 0 "/Game/EF_TwinsRoom/Common/Materials/Wood/WM_LaqueredBlackWood_a_Mat.WM_LaqueredBlackWood_a_Mat"))

(fn `UserConstructionScript`)