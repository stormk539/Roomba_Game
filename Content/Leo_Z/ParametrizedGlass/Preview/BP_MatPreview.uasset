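; Material preview actor for the ParametrizedGlass content that labels itself with a material instance name derived from its own display name.
; The construction script swaps the "Mat_Preview_" prefix for "MI_" and writes the result to a TextRender, without reading the mesh's material.
; WrapText uses SplitText to break the name at underscores and groups segments under a length limit, but joins groups with underscores rather than line breaks.
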(fn `Split Text`
  (params (`In Text` :type Text) (`Split On` :type Text :default "NSLOCTEXT(\"[F7B26B404FEEC6904297E8A5B2E5322F]\", \"9EC54CA04C3614F0F80542BC9A25BDAF\", \"_\")"))
  (returns (`Return Value` :type "Array of Text"))
  (locals (Result :type "Array of Text") (Text :type String))
  (bind _result (`local.Result`))
  (bind (_lefts _rights _returnvalue) (`KismetStringLibrary.Split` (`local.Text`) (`KismetTextLibrary.Conv_TextToString` `Split On`)))
  (bind _output_get (set `local.Text` (`KismetTextLibrary.Conv_TextToString` `In Text`)))
  (while (> (`KismetStringLibrary.Len` _output_get) 0)
    (if _returnvalue
      (`KismetArrayLibrary.Array_Add` _result (`KismetTextLibrary.Conv_StringToText` _lefts))
      (set `local.Text` _rights)
      (else
        (`KismetArrayLibrary.Array_Add` _result (`KismetTextLibrary.Conv_StringToText` (`local.Text`)))
        (set `local.Text` ""))))
  (return (`local.Result`)))

(fn `UserConstructionScript`
  (bind _return_value (`self.Wrap Text` (`KismetTextLibrary.Conv_StringToText` (`KismetStringLibrary.Replace` (`KismetSystemLibrary.GetDisplayName` self) "Mat_Preview_" "MI_"))))
  (`TextRenderComponent.K2_SetText` (`self.TextRender`) _return_value))

(fn `Wrap Text`
  (params (Text :type Text) (`Line Length` :type Integer :default 20))
  (returns (`Return Value` :type Text))
  (locals (`Text Out` :type String) (`Text Line` :type String))
  (bind _text_line (`local.Text Line`))
  (bind _text_line_2 (`local.Text Line`))
  (bind _text_out (`local.Text Out`))
  (bind _text_out_2 (`local.Text Out`))
  (bind _returnvalue (> (`KismetStringLibrary.Len` _text_line) 0))
  (bind _return_value (`self.Split Text` Text "_"))
  (for _array_element _return_value
    (bind _returnvalue_2 (`KismetTextLibrary.Conv_TextToString` _array_element))
    (if (and (>= (+ (`KismetStringLibrary.Len` _returnvalue_2) (`KismetStringLibrary.Len` _text_line)) `Line Length`) _returnvalue)
      (set `local.Text Out` (`KismetStringLibrary.Concat_StrStr` _text_out_2 (select `bool` (> (`KismetStringLibrary.Len` _text_out_2) 0) :`true` " \n_") (`local.Text Line`)))
      (set `local.Text Line` _returnvalue_2)
      (elif _returnvalue
        (set `local.Text Line` (`KismetStringLibrary.Concat_StrStr` (`local.Text Line`) "_" _returnvalue_2))
        (else
          (set `local.Text Line` _returnvalue_2)))))
  (if (and _returnvalue (> (`KismetStringLibrary.Len` (`local.Text Out`)) 0))
    (bind _output_get (set `local.Text Out` (`KismetStringLibrary.Concat_StrStr` _text_out " \n_" _text_line_2)))
    (else
      (set `local.Text Out` (`KismetStringLibrary.Concat_StrStr` _text_out _text_line_2))))
  (return (`KismetTextLibrary.Conv_StringToText` _output_get)))